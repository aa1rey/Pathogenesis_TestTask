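; BP_Storage is a test storage container that holds named items, each with a float and integer value, in an array of DA_Test objects.
; BeginPlay creates the requested number of empty slots, copies in preset assets, then adds a sample item, printing the contents along the way.
; AddItem reuses the first slot whose GetValues reports empty, or constructs and appends a new one.
; Display functions read through a bounds-checked getter.
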(event `self.ReceiveBeginPlay`
  ;[0 0 0] Creating specified amount of items
  (for _ (range (`self.Amount`))
    (bind _returnvalue (`|GenericCreateObject` "/Script/PathogenesisTestTask.DA_Test"))
    (`KismetArrayLibrary.Array_Add` (`self.Array`) _returnvalue))
  ;[0 0 0] Adding existing data assets and show them
  (for _array_element (`self.AssetsToAdd`)
    (bind (_str _flt _num) (`DA_Test.GetValues` _array_element))
    (`self.AddItem` _str _flt _num))
  (`KismetSystemLibrary.Delay` 2.0)
  (`self.Show All Items`)
  ;[0 0 0] Add custom data asset and show it
  (`KismetSystemLibrary.Delay` 1.0)
  (`self.AddItem` "MyCustomDataAsset" 3.14 10)
  (`KismetSystemLibrary.PrintString` "Item successfully added!" true true (struct :`R` 0.076965 :`G` 1.0 :`A` 1.0))
  (`KismetSystemLibrary.Delay` 5.0)
  (`self.Show All Items`))

(fn `AddItem`
  (params (Name :type String) (FloatValue :type "Float (double-precision)") (IntValue :type Integer))
  (returns (Success :type Boolean))
  (locals (bFoundEmpty :type Boolean :default false) (L_Index :type Integer))
  ;[0 0 0] Trying to find empty slot
  (for (_array_element _array_index) (`self.Array`)
    (set `local.L_Index` _array_index)
    (if (not (`.ReturnValue` (`DA_Test.GetValues` _array_element)))
      (set `local.bFoundEmpty` true)
      (break)))
  (if (`local.bFoundEmpty`)
    ;[0 0 0] If empty slot exists - set values
    (`DA_Test.SetValues` (`|GetArrayItem` (`self.Array`) (`local.L_Index`)) (`local.Name`) (`local.FloatValue`) (`local.IntValue`))
    (return true)
    (else
      ;[0 0 0] If empty slot doesn't exist - add new slot and set values
      (bind _returnvalue (`|GenericCreateObject` "/Script/PathogenesisTestTask.DA_Test"))
      (`KismetArrayLibrary.Array_Add` (`self.Array`) _returnvalue)
      (`DA_Test.SetValues` _returnvalue (`local.Name`) (`local.FloatValue`) (`local.IntValue`))
      (return true))))

(fn `GetItemAtIndex`
  (params (Index :type Integer))
  (returns (Success :type Boolean) (str :type String) (flt :type "Float (single-precision)") (num :type Integer))
  (bind (_str _flt _num _returnvalue) (`DA_Test.GetValues` (`|GetArrayItem` (`self.Array`) (`local.Index`))))
  (if (`KismetArrayLibrary.Array_IsValidIndex` (`self.Array`) Index)
    (return _returnvalue _str _flt _num)
    (else
      (return false "" 0.0 0))))

(fn `Show All Items`
  (for (_ _array_index) (`self.Array`)
    (`self.Show Item at Index` _array_index))
  (return))

(fn `Show Item at Index`
  (params (Index :type Integer))
  (bind (_success _str _flt _num) (`self.GetItemAtIndex` Index))
  (if _success
    (`KismetSystemLibrary.PrintString` (`KismetStringLibrary.Concat_StrStr` "Name: " _str " | Float Val: " (`KismetStringLibrary.Conv_DoubleToString` _flt) " | Int Val: " (`KismetStringLibrary.Conv_IntToString` _num)) true true (struct :`R` 1.0 :`G` 0.926017 :`A` 1.0) 5.0))
  (return))

(fn `UserConstructionScript`)