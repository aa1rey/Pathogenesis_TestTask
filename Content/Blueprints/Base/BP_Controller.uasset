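; BP_Controller is the player controller that creates the main HUD and pause menu widgets and manages cursor, input mode and pausing.
; It binds to the PlayerCharacter's inventory visibility, orient-to-mouse and pause delegates, plus the pause menu's continue event, which toggles pause back through the character.
; While mouse orientation is active, a looping timer traces under the cursor and yaws the character mesh toward the hit point, suspending orient-to-movement.
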(event `self.ReceiveBeginPlay`
  (`|ExecutionSequence`
    (:`then_0`
      ;[0 0 0] Add widgets to viewport
      (bind _returnvalue (`|CreateWidget` "/Game/Blueprints/UI/WBP_Main.WBP_Main_C" self))
      (bind _output_get (set `self.MainWidget` _returnvalue))
      (`UserWidget.AddToViewport` _output_get 998)
      (bind _returnvalue_2 (`|CreateWidget` "/Game/Blueprints/UI/WBP_PauseMenu.WBP_PauseMenu_C" self))
      (bind _output_get_2 (set `self.PauseWidget` _returnvalue_2))
      (`UserWidget.AddToViewport` _output_get_2 999))
    (:`then_1`
      ;[0 0 0] Bind delegates
      (bind _asplayer_character (cast `PlayerCharacter` (`self.K2_GetPawn`)))
      (bind _output_get_3 (set `self.PlayerRef` _asplayer_character))
      (add `InventoryComponent.OnInventoryVisibilityUpdate` (`PlayerCharacter.GetInventory` _output_get_3) (`|CreateDelegate` :!event `OnInventoryVisibilityUpdate`))
      (add `PlayerCharacter.OnOrientToMousePosition` (`self.PlayerRef`) (`|CreateDelegate` :!event `OnOrientToMousePosition`))
      (add `PlayerCharacter.OnPause` (`self.PlayerRef`) (`|CreateDelegate` :!event `OnPause`))
      (add `/Game/Blueprints/UI/WBP_PauseMenu.OnGameContinue` (`self.PauseWidget`) (`|CreateDelegate` :!event `OnGameContinue`)))))

(event `OnInventoryVisibilityUpdate`
  (params (`bVisible?` :type Boolean))
  ;[0 0 0] Inventory widget visibility
  (bind _output_get (set `self.bShowMouseCursor` `bVisible?`))
  (`/Game/Blueprints/UI/WBP_Main.OnInventoryVisibilityUpdate` (`self.MainWidget`) _output_get)
  (`self.Set Input Mode` (`self.bShowMouseCursor`)))

(event `OnOrientToMousePosition`
  (params (bOrient :type Boolean))
  ;[0 0 0] Orient Player to mouse position
  (if bOrient
    (bind _returnvalue (`KismetSystemLibrary.K2_SetTimerDelegate` (`|CreateDelegate` :!event `OrientToMousePosition`) 0.01 true))
    (set `self.OrientToMouseHandle` _returnvalue)
    (set `self.bShowMouseCursor` true)
    (set `CharacterMovementComponent.bOrientRotationToMovement` false (`Character.CharacterMovement` (`self.PlayerRef`)))
    (`WidgetBlueprintLibrary.SetInputMode_GameAndUIEx` self null "DoNotLock" false)
    (else
      (`self.EndOrientToMouse`)
      (`WidgetBlueprintLibrary.SetInputMode_GameOnly` self))))

(event `EndOrientToMouse`
  ;[0 0 0] Orient Player to mouse position
  (`KismetSystemLibrary.K2_ClearAndInvalidateTimerHandle` (`self.OrientToMouseHandle`))
  (set `self.bShowMouseCursor` false)
  (bind _playerref (`self.PlayerRef`)
    (:`then`
      (set `CharacterMovementComponent.bOrientRotationToMovement` true (`Character.CharacterMovement` _playerref)))
    (:`else`)))

(event `OrientToMousePosition`
  (bind (_hitresult _returnvalue) (`self.GetHitResultUnderCursorForObjects` (`|MakeArray` "ObjectTypeQuery1" "ObjectTypeQuery2" "ObjectTypeQuery3" :!type "EObjectTypeQuery Enum") false))
  (bind (_returnvalue_roll _returnvalue_pitch) (`KismetMathLibrary.BreakRotator` (`SceneComponent.K2_GetComponentRotation` (`Character.Mesh` (`self.PlayerRef`)))))
  (bind (_returnvalue_roll_2 _returnvalue_pitch_2 _returnvalue_yaw) (`KismetMathLibrary.BreakRotator` (`KismetMathLibrary.FindLookAtRotation` (`self.K2_GetActorLocation` (`self.PlayerRef`)) (`.ImpactPoint` (`GameplayStatics.BreakHitResult` _hitresult)))))
  ;[0 0 0] Orient Player to mouse position
  (`self.PlayerRef`
    (:`then`
      (if _returnvalue
        (`SceneComponent.K2_SetWorldRotation` (`Character.Mesh` (`self.PlayerRef`)) (`KismetMathLibrary.MakeRotator` _returnvalue_roll _returnvalue_pitch (- _returnvalue_yaw 90.0)) false false)))
    (:`else`
      (`self.EndOrientToMouse`))))

(event `OnPause`
  (params (bPause :type Boolean))
  ;[0 0 0] Pause Game
  (bind _output_get (set `self.bShowMouseCursor` bPause))
  (`self.Set Input Mode` _output_get)
  (`Widget.SetVisibility` (`self.PauseWidget`) (select `bool` (`self.bShowMouseCursor`) :`false` "Hidden" :`true` "SelfHitTestInvisible" :!type "ESlateVisibility Enum"))
  (`GameplayStatics.SetGamePaused` (`self.bShowMouseCursor`)))

(event `OnGameContinue`
  ;[0 0 0] Pause Game
  (`PlayerCharacter.TogglePause` (`self.PlayerRef`)))

(fn `Set Input Mode`
  (params (Condition :type Boolean))
  (if Condition
    (`WidgetBlueprintLibrary.SetInputMode_GameAndUIEx` self null "DoNotLock" false)
    (else
      (`WidgetBlueprintLibrary.SetInputMode_GameOnly` self)))
  (return))

(fn `UserConstructionScript`)