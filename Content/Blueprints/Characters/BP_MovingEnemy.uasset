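; BP_MovingEnemy is an enemy character Blueprint that connects its health component to a health bar widget.
; On BeginPlay it runs the parent logic, casts the HealthWidget's widget to WBP_HealthBar, caches it, and copies in the component's max health.
; It then binds an event to the component's current-health update; no movement logic or handler body appears in these graphs.
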(event `self.ReceiveBeginPlay`
  (`parent.ReceiveBeginPlay`)
  (bind _aswbp_health_bar (cast `/Game/Blueprints/UI/WBP_HealthBar` (`WidgetComponent.GetWidget` (`self.HealthWidget`))))
  (set `self.WHealth` _aswbp_health_bar)
  (set `/Game/Blueprints/UI/WBP_HealthBar.MaxHealth` (`HealthComponent.GetMaxHealth` (`self.HealthComponent`)) (`self.WHealth`))
  (add `HealthComponent.OnCurrentHealthUpdate` (`self.HealthComponent`) (`|CreateDelegate` (`self.WHealth`) :!event `SetBarPersent`)))

(fn `UserConstructionScript`)